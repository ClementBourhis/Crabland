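; BP_Shroom is a foliage mushroom actor with configurable colors for its curved mesh and Niagara spores.
; On BeginPlay it sets base and subsurface colors on a dynamic material and passes the spore color to Niagara.
; It creates both dynamic materials from slot 1's material on slot 0, so the second, carrying only emissive color, replaces the first.
; Construction script is empty.
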(event `self.ReceiveBeginPlay`
  (bind _longcurvedshroom (`self.LongCurvedShroom`))
  (bind _longcurvedshroom_2 (`self.LongCurvedShroom`))
  (bind _returnvalue (`PrimitiveComponent.CreateDynamicMaterialInstance` _longcurvedshroom_2 0 (`PrimitiveComponent.GetMaterial` _longcurvedshroom_2 1) "None"))
  (`MaterialInstanceDynamic.SetVectorParameterValue` _returnvalue "BaseColor" (`KismetMathLibrary.Conv_ColorToLinearColor` (`self.Color`)))
  (`MaterialInstanceDynamic.SetVectorParameterValue` _returnvalue "SubSurfaceScat" (`KismetMathLibrary.Conv_ColorToLinearColor` (`self.SubsurfaceColor`)))
  (`FXSystemComponent.SetColorParameter` (`self.NS_SporesShroom`) "Color" (`KismetMathLibrary.Conv_ColorToLinearColor` (`self.SporesColors`)))
  (bind _returnvalue_2 (`PrimitiveComponent.CreateDynamicMaterialInstance` _longcurvedshroom 0 (`PrimitiveComponent.GetMaterial` _longcurvedshroom 1) "None"))
  (`MaterialInstanceDynamic.SetVectorParameterValue` _returnvalue_2 "EmissiveColor" (`KismetMathLibrary.Conv_ColorToLinearColor` (`self.EmissiveColors`))))

(fn `UserConstructionScript`)